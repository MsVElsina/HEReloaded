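; Horror Engine component that saves and loads the game through separate "Level" and "Player" HE_SaveGame slots.
; Saving stores the level name plus player transform, items, quest, device life and ammo.
; Loading flags HE_GameInstance and reopens the level, so BeginPlay then restores the player.
; Restoring replays Use on saved items, seeks device timelines to their remaining life and re-equips active gear.
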(event Custom|SavePlayer
  (bind _player (Variables|Default|GetPlayer))
  (bind _saveplayerref (Variables|Default|GetSavePlayerRef))
  ;[1 1 1] Save And Load Player
  (Utilities|CallPlayerSlot)
  (Variables|/Game/HorrorEngine/Blueprints/Core/HE_SaveGame.HE_SaveGame_C|SetInventory (Variables|Default|GetSavePlayerRef) (Variables|/Game/HorrorEngine/HorrorEngine.HorrorEngine_C|GetPlayerInventory (Variables|Default|GetPlayer)))
  (Variables|/Game/HorrorEngine/Blueprints/Core/HE_SaveGame.HE_SaveGame_C|SetEquipment (Variables|Default|GetSavePlayerRef) (Variables|/Game/HorrorEngine/HorrorEngine.HorrorEngine_C|GetPlayerEquipment (Variables|Default|GetPlayer)))
  (Variables|/Game/HorrorEngine/Blueprints/Core/HE_SaveGame.HE_SaveGame_C|SetPlayerTransform (Variables|Default|GetSavePlayerRef) (Math|Transform|MakeTransform (Transformation|GetWorldLocation (Variables|/Script/Engine.Character|GetCapsuleComponent (Game|GetPlayerCharacter 0))) (Pawn|GetControlRotation (Game|GetPlayerController 0) :!class /Script/Engine.Controller) "1,1,1"))
  (Variables|/Game/HorrorEngine/Blueprints/Core/HE_SaveGame.HE_SaveGame_C|SetPlayerQuest _saveplayerref (Variables|/Game/HorrorEngine/Blueprints/Core/Inspectable.Inspectable_C|GetItemInformation (Variables|/Game/HorrorEngine/HorrorEngine.HorrorEngine_C|GetDiary _player)))
  (Variables|/Game/HorrorEngine/Blueprints/Core/HE_SaveGame.HE_SaveGame_C|SetGlowstickRemainingLife%20%28%25%29 _saveplayerref (Variables|/Game/HorrorEngine/HorrorEngine.HorrorEngine_C|GetGlowstickRemainingLife%20%28%25%29 _player))
  (Variables|/Game/HorrorEngine/Blueprints/Core/HE_SaveGame.HE_SaveGame_C|SetFlashlightRemainingBattery%20%28%25%29 _saveplayerref (Variables|/Game/HorrorEngine/HorrorEngine.HorrorEngine_C|GetFlashlightRemainingBattery%20%28%25%29 _player))
  (Variables|/Game/HorrorEngine/Blueprints/Core/HE_SaveGame.HE_SaveGame_C|SetLighterRemainingLife%20%28%25%29 _saveplayerref (Variables|/Game/HorrorEngine/HorrorEngine.HorrorEngine_C|GetLighterRemainingLife%20%28%25%29 _player))
  (Variables|/Game/HorrorEngine/Blueprints/Core/HE_SaveGame.HE_SaveGame_C|SetTorchRemainingLife%20%28%25%29 _saveplayerref (Variables|/Game/HorrorEngine/HorrorEngine.HorrorEngine_C|GetTorchRemainingLife%20%28%25%29 _player))
  (Variables|/Game/HorrorEngine/Blueprints/Core/HE_SaveGame.HE_SaveGame_C|SetNightVisionRemainingBattery%20%28%25%29 _saveplayerref (Variables|/Game/HorrorEngine/HorrorEngine.HorrorEngine_C|GetNightVisionRemainingBattery%20%28%25%29 _player))
  (Variables|/Game/HorrorEngine/Blueprints/Core/HE_SaveGame.HE_SaveGame_C|SetNightVisionCurrentFOV _saveplayerref (Variables|/Game/HorrorEngine/HorrorEngine.HorrorEngine_C|GetNightVisionCurrentFOV _player))
  (Variables|/Game/HorrorEngine/Blueprints/Core/HE_SaveGame.HE_SaveGame_C|SetPistolTotalAmmo _saveplayerref (Variables|/Game/HorrorEngine/HorrorEngine.HorrorEngine_C|GetPistolTotalAmmo _player))
  (Variables|/Game/HorrorEngine/Blueprints/Core/HE_SaveGame.HE_SaveGame_C|SetPistolClipAmmo _saveplayerref (Variables|/Game/HorrorEngine/HorrorEngine.HorrorEngine_C|GetPistolClipAmmo _player))
  (Variables|/Game/HorrorEngine/Blueprints/Core/HE_SaveGame.HE_SaveGame_C|SetGlowstickOff _saveplayerref (Variables|/Game/HorrorEngine/HorrorEngine.HorrorEngine_C|GetGlowstickOff _player))
  (Variables|/Game/HorrorEngine/Blueprints/Core/HE_SaveGame.HE_SaveGame_C|SetFlashlightOff _saveplayerref (Variables|/Game/HorrorEngine/HorrorEngine.HorrorEngine_C|GetFlashlightOff _player))
  (Variables|/Game/HorrorEngine/Blueprints/Core/HE_SaveGame.HE_SaveGame_C|SetLighterOff _saveplayerref (Variables|/Game/HorrorEngine/HorrorEngine.HorrorEngine_C|GetLighterOff _player))
  (Variables|/Game/HorrorEngine/Blueprints/Core/HE_SaveGame.HE_SaveGame_C|SetTorchOff _saveplayerref (Variables|/Game/HorrorEngine/HorrorEngine.HorrorEngine_C|GetTorchOff _player))
  (Variables|/Game/HorrorEngine/Blueprints/Core/HE_SaveGame.HE_SaveGame_C|SetNightVisionOff _saveplayerref (Variables|/Game/HorrorEngine/HorrorEngine.HorrorEngine_C|GetNightVisionOff _player))
  (Variables|/Game/HorrorEngine/Blueprints/Core/HE_SaveGame.HE_SaveGame_C|SetPistolOff _saveplayerref (Variables|/Game/HorrorEngine/HorrorEngine.HorrorEngine_C|GetPistolOff _player))
  (SaveGame|SaveGametoSlot (Variables|Default|GetSavePlayerRef) "Player"))

(event Custom|LoadLevel
  ;[1 1 1] Save And Load Level
  (Variables|/Game/HorrorEngine/Blueprints/Core/HE_GameInstance.HE_GameInstance_C|SetLoading (Variables|Default|GetGameInstance) true)
  (Utilities|CallLevelSlot)
  (Game|OpenLevel(byName) (Utilities|String|StringToName (Variables|/Game/HorrorEngine/Blueprints/Core/HE_SaveGame.HE_SaveGame_C|GetLevelName (Variables|Default|GetSaveLevelRef)))))

(event Custom|SaveLevel
  ;[1 1 1] Save And Load Level
  (Utilities|CallLevelSlot)
  (bind _returnvalue (Game|GetCurrentLevelName true))
  (Variables|/Game/HorrorEngine/Blueprints/Core/HE_SaveGame.HE_SaveGame_C|SetLevelName (Variables|Default|GetSaveLevelRef) _returnvalue)
  (SaveGame|SaveGametoSlot (Variables|Default|GetSaveLevelRef) "Level"))

(event Custom|SaveGame
  ;[1 1 1] Main Save and Load Command
  (CallFunction|SaveLevel)
  (CallFunction|SavePlayer)
  (CallFunction|Notice "" "Game Saved"))

(event Custom|LoadGame
  ;[1 1 1] Main Save and Load Command
  (CallFunction|LoadLevel))

(event Custom|LoadPlayer
  (bind _player (Variables|Default|GetPlayer))
  (bind _player_2 (Variables|Default|GetPlayer))
  (bind _saveplayerref (Variables|Default|GetSavePlayerRef))
  (bind _saveplayerref_2 (Variables|Default|GetSavePlayerRef))
  (bind _saveplayerref_3 (Variables|Default|GetSavePlayerRef))
  (bind _playertransform (Variables|/Game/HorrorEngine/Blueprints/Core/HE_SaveGame.HE_SaveGame_C|GetPlayerTransform _saveplayerref_3))
  ;[1 1 1] Save And Load Player
  (Utilities|CallPlayerSlot)
  (Transformation|SetWorldLocation (Variables|/Script/Engine.Character|GetCapsuleComponent (Game|GetPlayerCharacter 0)) (.location _playertransform) false false)
  (Pawn|SetControlRotation (Game|GetPlayerController 0) (.rotation _playertransform))
  (for _array_element (Variables|/Game/HorrorEngine/Blueprints/Core/HE_SaveGame.HE_SaveGame_C|GetInventory (Variables|Default|GetSavePlayerRef))
    (bind _asinspectable (Utilities|Casting|CastToInspectable _array_element))
    (Default|Use _asinspectable false))
  (for _array_element_2 (Variables|/Game/HorrorEngine/Blueprints/Core/HE_SaveGame.HE_SaveGame_C|GetEquipment (Variables|Default|GetSavePlayerRef))
    (bind _asinspectable_2 (Utilities|Casting|CastToInspectable _array_element_2))
    (Default|Use _asinspectable_2 false))
  (for (_array_element_3 _array_index) (Utilities|Array|MakeArray (Variables|/Game/HorrorEngine/HorrorEngine.HorrorEngine_C|GetGlowstickDurationTimeline _player_2) (Variables|/Game/HorrorEngine/HorrorEngine.HorrorEngine_C|GetFlashlightDurationTimeline _player_2) (Variables|/Game/HorrorEngine/HorrorEngine.HorrorEngine_C|GetLighterDurationTimeline _player_2) (Variables|/Game/HorrorEngine/HorrorEngine.HorrorEngine_C|GetTorchDurationTimeline _player_2) (Variables|/Game/HorrorEngine/HorrorEngine.HorrorEngine_C|GetNightVisionDurationTimeline _player_2))
    (Components|Timeline|SetNewTime _array_element_3 (Math|Float|Lerp 6e+01 0.0 (/ (Utilities|Select :Index _array_index :Option%200 (Variables|/Game/HorrorEngine/Blueprints/Core/HE_SaveGame.HE_SaveGame_C|GetGlowstickRemainingLife%20%28%25%29 _saveplayerref_2) :Option%201 (Variables|/Game/HorrorEngine/Blueprints/Core/HE_SaveGame.HE_SaveGame_C|GetFlashlightRemainingBattery%20%28%25%29 _saveplayerref_2) :Option%202 (Variables|/Game/HorrorEngine/Blueprints/Core/HE_SaveGame.HE_SaveGame_C|GetLighterRemainingLife%20%28%25%29 _saveplayerref_2) :Option%203 (Variables|/Game/HorrorEngine/Blueprints/Core/HE_SaveGame.HE_SaveGame_C|GetTorchRemainingLife%20%28%25%29 _saveplayerref_2) :Option%204 (Variables|/Game/HorrorEngine/Blueprints/Core/HE_SaveGame.HE_SaveGame_C|GetNightVisionRemainingBattery%20%28%25%29 _saveplayerref_2)) 1e+02))))
  (Variables|/Game/HorrorEngine/Blueprints/Core/Inspectable.Inspectable_C|SetItemInformation (Variables|/Game/HorrorEngine/HorrorEngine.HorrorEngine_C|GetDiary _player) (Variables|/Game/HorrorEngine/Blueprints/Core/HE_SaveGame.HE_SaveGame_C|GetPlayerQuest _saveplayerref))
  (Variables|/Game/HorrorEngine/HorrorEngine.HorrorEngine_C|SetNightVisionCurrentFOV _player (Variables|/Game/HorrorEngine/Blueprints/Core/HE_SaveGame.HE_SaveGame_C|GetNightVisionCurrentFOV _saveplayerref))
  (Variables|/Game/HorrorEngine/HorrorEngine.HorrorEngine_C|SetPistolTotalAmmo _player (Variables|/Game/HorrorEngine/Blueprints/Core/HE_SaveGame.HE_SaveGame_C|GetPistolTotalAmmo _saveplayerref))
  (Variables|/Game/HorrorEngine/HorrorEngine.HorrorEngine_C|SetPistolClipAmmo _player (Variables|/Game/HorrorEngine/Blueprints/Core/HE_SaveGame.HE_SaveGame_C|GetPistolClipAmmo _saveplayerref))
  (Utilities|RestoreEquipment))

(event EventBeginPlay
  ;[1 1 1] After Load Level
  (bind _asmaster (CallFunction|GetPlayer))
  (Variables|Default|SetPlayer _asmaster)
  (bind _ashe_game_instance (Utilities|Casting|CastToHE_GameInstance (Game|GetGameInstance))
    (:then
      (Variables|Default|SetGameInstance _ashe_game_instance)
      (if (Variables|/Game/HorrorEngine/Blueprints/Core/HE_GameInstance.HE_GameInstance_C|GetLoading (Variables|Default|GetGameInstance))
        (CallFunction|LoadPlayer)
        (Variables|/Game/HorrorEngine/Blueprints/Core/HE_GameInstance.HE_GameInstance_C|SetLoading (Variables|Default|GetGameInstance) false)
        (Utilities|FlowControl|Delay 0.2)
        (CallFunction|Notice "" "Game Loaded")))
    (:CastFailed
      (Development|PrintString "Set Game Instance Class as \"HE_GameInstance\" from Project Settings / Maps&Modes." true true "(R=0.000000,G=0.660000,B=1.000000,A=1.000000)" 5.0))))