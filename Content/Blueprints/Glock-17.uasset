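; Glock-17 weapon Blueprint that plays the pistol's skeletal mesh animations for its handling states.
; Separate events for draw, hide, fire-mode switch, idle, reload and shot each play a matching animation once, without looping, directly on the mesh.
; It holds no firing, ammo or state logic, and its construction script is empty.
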(event Custom|Shot
  (Components|Animation|PlayAnimation (Variables|Default|GetSkeletalMesh) "/Game/BarcodeWeapons/BarcodeGamesPistol/source/Glock-17_Anim_Shoot.Glock-17_Anim_Shoot" false))

(event Custom|Draw
  (Components|Animation|PlayAnimation (Variables|Default|GetSkeletalMesh) "/Game/BarcodeWeapons/BarcodeGamesPistol/source/Glock-17_Anim_Draw.Glock-17_Anim_Draw" false))

(event Custom|Hide
  (Components|Animation|PlayAnimation (Variables|Default|GetSkeletalMesh) "/Game/BarcodeWeapons/BarcodeGamesPistol/source/Glock-17_Anim_Hide.Glock-17_Anim_Hide" false))

(event Custom|Firemode
  (Components|Animation|PlayAnimation (Variables|Default|GetSkeletalMesh) "/Game/BarcodeWeapons/BarcodeGamesPistol/source/fireswitch.fireswitch" false))

(event Custom|Idle
  (Components|Animation|PlayAnimation (Variables|Default|GetSkeletalMesh) "/Game/BarcodeWeapons/BarcodeGamesPistol/source/Glock-17_Anim_Idle.Glock-17_Anim_Idle" false))

(event Custom|Reload
  (Components|Animation|PlayAnimation (Variables|Default|GetSkeletalMesh) "/Game/BarcodeWeapons/BarcodeGamesPistol/source/Glock-17_Anim_Reload.Glock-17_Anim_Reload" false))

(fn ConstructionScript)