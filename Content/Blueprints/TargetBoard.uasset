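; Target board actor that keeps a running damage total and shows it on a text render.
; Separate head and chest hitboxes each add their own hit value on begin overlap, if the overlapping actor carries the required actor tag.
; Both hits then call Updatedamage, which refreshes the displayed total and prints a debug "Hit" message.
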(event OnComponentBeginOverlap(Chesthitbox)
  (params (OverlappedComponent :type Primitive%20Component%20Object%20Reference) (OtherActor :type Actor%20Object%20Reference) (OtherComp :type Primitive%20Component%20Object%20Reference) (OtherBodyIndex :type Integer) (bFromSweep :type Boolean) (SweepResult :type Hit%20Result%20Structure%20%28by%20ref%29))
  ;[1 1 1] Chest Hit
  (if (Actor|ActorHasTag OtherActor "GetFucked")
    (Variables|Default|SetDamVal (+ (Variables|Default|GetDamVal) (Variables|Default|GetChestHit)))
    (CallFunction|Updatedamage)))

(event OnComponentBeginOverlap(HeadHitbox)
  (params (OverlappedComponent :type Primitive%20Component%20Object%20Reference) (OtherActor :type Actor%20Object%20Reference) (OtherComp :type Primitive%20Component%20Object%20Reference) (OtherBodyIndex :type Integer) (bFromSweep :type Boolean) (SweepResult :type Hit%20Result%20Structure%20%28by%20ref%29))
  ;[1 1 1] Head Hit
  (if (Actor|ActorHasTag OtherActor "GetFucked")
    (Variables|Default|SetDamVal (+ (Variables|Default|GetDamVal) (Variables|Default|GetHeadHit)))
    (CallFunction|Updatedamage)))

(event Custom|Updatedamage
  (Rendering|Components|TextRender|SetText (Variables|Default|GetTextRender) (Utilities|Text|ToText(Integer) (Variables|Default|GetDamVal)))
  (Development|PrintString "Hit"))

(event EventBeginPlay)

(event Collision|EventActorBeginOverlap
  (params (OtherActor :type Actor%20Object%20Reference)))

(fn ConstructionScript)